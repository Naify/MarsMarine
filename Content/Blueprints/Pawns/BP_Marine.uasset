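; Player marine for a twin-stick style shooter, with world-axis movement, a HUD, health, death and a kill counter.
; Each tick it sets control yaw from smoothed mouse velocity or thumbstick direction, both with deadzones, based on whether the last key pressed was a keyboard key.
; Firing runs looping audio, muzzle effects and a timer-repeated line trace from the rifle muzzle along control rotation, applying damage and spawning impact effects.
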(event `self.ReceiveAnyDamage`
  (params (Damage :type "Float (single-precision)") (DamageType :type "DamageType Object Reference") (InstigatedBy :type "Controller Object Reference") (DamageCauser :type "Actor Object Reference"))
  (bind _health (`self.Decreasehealth` Damage))
  (if (== _health 0.0)
    (set `self.Dead` true)
    (`self.StopFiringWeapon`)))

(event `self.ReceiveBeginPlay`
  (bind _returnvalue (`|CreateWidget` "/Game/UI/W_PlayerHUD.W_PlayerHUD_C" null self))
  (`UserWidget.AddToViewport` _returnvalue 0))

(event `InputAction|FIreWeapon`
  (params (Key :type "Key Structure"))
  (:`Pressed`
    (`self.StartFiringWeapon`))
  (:`Released`
    (`self.StopFiringWeapon`)))

(event `Key|AnyKey`
  (params (Key :type "Key Structure"))
  (:`Pressed`
    (set `self.KeyboardActive` (`KismetInputLibrary.Key_IsKeyboardKey` Key))))

(event `InputAxis|MoveForward`
  (params (AxisValue :type "Float (single-precision)"))
  (if (`self.IsAlive`)
    (`self.AddMovementInput` (1.0 0.0 0.0) AxisValue)))

(event `InputAxis|MoveRight`
  (params (AxisValue :type "Float (single-precision)"))
  (if (`self.IsAlive`)
    (`self.AddMovementInput` (0.0 1.0 0.0) AxisValue)))

(event `self.ReceiveTick`
  (params (DeltaSeconds :type "Float (single-precision)"))
  (`self.UpdatePlayerAim`))

(fn `AddHealth`
  (params (healthToAdd :type "Float (double-precision)"))
  (set `self.Health` (`KismetMathLibrary.FClamp` (+ (`self.Health`) healthToAdd) 0.0 100.0)))

(fn `Decreasehealth`
  (params (B :type "Float (double-precision)"))
  (returns (Health :type "Float (double-precision)"))
  (bind _output_get (set `self.Health` (`KismetMathLibrary.FClamp` (- (`self.Health`) B) 0.0 100.0)))
  (return _output_get))

(fn `GetMouseAimDirection`
  (returns (ReturnValue :type "Rotator Structure"))
  (bind (_returnvalue_x _returnvalue_y) (`KismetMathLibrary.BreakVector2D` (`self.GetMouseVelocity`)))
  (return (`KismetMathLibrary.RInterpTo` (`Controller.GetControlRotation` (`GameplayStatics.GetPlayerController` 0)) (`KismetMathLibrary.MakeRotator` 0.0 0.0 (`KismetMathLibrary.DegAtan2` _returnvalue_y _returnvalue_x)) (`GameplayStatics.GetWorldDeltaSeconds`) (`self.MouseSmoothingStrength`))))

(fn `GetMouseVelocity`
  (returns (ReturnValue :type "Vector2D Structure"))
  (bind (_deltax _deltay) (`PlayerController.GetInputMouseDelta` (`GameplayStatics.GetPlayerController` 0)))
  (return (/ (`KismetMathLibrary.MakeVector2D` _deltax _deltay) (`GameplayStatics.GetWorldDeltaSeconds`))))

(fn `GetThumbAimDirection`
  (returns (ReturnValue :type "Rotator Structure"))
  (return (`KismetMathLibrary.MakeRotator` 0.0 0.0 (`KismetMathLibrary.DegAtan2` (`self.GetInputAxisValue`) (`self.GetInputAxisValue`)))))

(fn `GetWeaponEndLocation`
  (returns (ReturnValue :type "Vector Structure"))
  (return (+ (`self.GetWeaponStartLocation`) (* (`KismetMathLibrary.GetForwardVector` (`self.GetControlRotation`)) (`self.WeaponRange`)))))

(fn `GetWeaponStartLocation`
  (returns (ReturnValue :type "Vector Structure"))
  (return (`SceneComponent.GetSocketLocation` (`self.Rifle`) "MuzzleFlashSocket")))

(fn `IncreaseKills`
  (`/Engine/EditorBlueprintResources/StandardMacros.IncrementInt` (`self.Kills`)))

(fn `IsAlive`
  (returns (ReturnValue :type Boolean))
  (return (not (`self.Dead`))))

(fn `IsHealthFull`
  (returns (ReturnValue :type Boolean))
  (return (== (`self.Health`) 100.0)))

(fn `IsMouseAboveDeadzone`
  (returns (Output_Get :type Boolean))
  (locals (NewLocalVar_0 :type "Float (double-precision)" :default 0.0))
  (return (> (`KismetMathLibrary.VSize2D` (`self.GetMouseVelocity`)) (`self.MouseDeadzone`))))

(fn `IsThumbAboveDeadzone`
  (returns (ReturnValue :type Boolean))
  (return (> (`KismetMathLibrary.VSize2D` (`KismetMathLibrary.MakeVector2D` (`self.GetInputAxisValue`) (`self.GetInputAxisValue`))) (`self.ThumbstickDeadzone`))))

(fn `SpawnImpactHit`
  (params (HitLocation :type "Vector Structure"))
  (`GameplayStatics.SpawnEmitterAtLocation` "/Game/Effects/Weapons/Impacts/P_AssaultRifle_IH.P_AssaultRifle_IH" HitLocation))

(fn `StartFiringWeapon`
  (if (`self.IsAlive`)
    (`ActorComponent.Activate` (`self.P_AssaultRifle_MF`) false)
    (bind _returnvalue (`GameplayStatics.SpawnSound2D` "/Game/Sounds/Weapon_AssaultRifle/Stereo/RifleFireLoopCue.RifleFireLoopCue" 1.0 1.0 0.0 null))
    (set `self.WeaponFireSound` _returnvalue)
    (`self.WeaponTrace`)
    (`KismetSystemLibrary.K2_SetTimer` null "WeaponTrace" (`self.WeaponFireRate`) true)))

(fn `StopFiringWeapon`
  (`ActorComponent.Deactivate` (`self.P_AssaultRifle_MF`))
  (`AudioComponent.Stop` (`self.WeaponFireSound`))
  (`KismetSystemLibrary.K2_ClearTimer` null "WeaponTrace")
  (if (`self.IsAlive`)
    (`GameplayStatics.SpawnSound2D` "/Game/Sounds/Weapon_AssaultRifle/Stereo/RifleFireEnd_cue.RifleFireEnd_cue" 1.0 1.0 0.0 null)))

(fn `UpdateMouseAim`
  (if (`self.IsMouseAboveDeadzone`)
    (`Controller.SetControlRotation` (`GameplayStatics.GetPlayerController` 0) (`self.GetMouseAimDirection`))))

(fn `UpdatePlayerAim`
  (if (`self.IsAlive`)
    (if (`self.KeyboardActive`)
      (`self.UpdateMouseAim`)
      (else
        (`self.UpdateThumbAim`)))))

(fn `UpdateThumbAim`
  (if (`self.IsThumbAboveDeadzone`)
    (`Controller.SetControlRotation` (`GameplayStatics.GetPlayerController` 0) (`self.GetThumbAimDirection`))))

(fn `UserConstructionScript`)

(fn `WeaponTrace`
  (bind _outhit (`KismetSystemLibrary.LineTraceSingle` (`self.GetWeaponStartLocation`) (`self.GetWeaponEndLocation`) "TraceTypeQuery1"))
  (bind (_bblockinghit _binitialoverlap _time _distance _location _impactpoint _normal _impactnormal _physmat _hitactor) (`GameplayStatics.BreakHitResult` _outhit))
  (if _bblockinghit
    (`self.SpawnImpactHit` _location)
    (`GameplayStatics.ApplyDamage` _hitactor (`self.DamagePerShot`))))